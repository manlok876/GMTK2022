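; BP_ChessBoard is a board Blueprint that maps row and column cell coordinates to positions on a grid.
; GetCellOffset centers the grid on the origin using Rows and Columns, then scales by CellSize, with rows along X and columns along Y.
; GetPositionForCell turns that 2D offset into a vector at zero Z, without applying the actor's transform.
; The event graph and construction script are empty.
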(fn `GetCellOffset`
  (params (Coords :type "GridCoords Structure"))
  (returns (ReturnValue :type "Vector2D Structure"))
  (return (* (- (`KismetMathLibrary.MakeVector2D` (`KismetMathLibrary.Conv_IntToDouble` Coords_Row) (`KismetMathLibrary.Conv_IntToDouble` Coords_Column)) (/ (- (`KismetMathLibrary.MakeVector2D` (`KismetMathLibrary.Conv_IntToDouble` (`self.Rows`)) (`KismetMathLibrary.Conv_IntToDouble` (`self.Columns`))) 1.0) 2.0)) (`self.CellSize`))))

(fn `GetPositionForCell`
  (params (Coords :type "GridCoords Structure"))
  (returns (Result :type "Vector Structure"))
  (bind _returnvalue (`self.GetCellOffset` Coords))
  (return (`KismetMathLibrary.Conv_Vector2DToVector` _returnvalue)))

(fn `UserConstructionScript`)