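; Chess piece actor with figure and dice meshes that forwards clicks to BP_PlayerController.
; Type or color changes update the dice mesh and apply opposite-colored materials to figure and die; the figure-mesh update is never called.
; A timeline moves it between BP_ChessBoard cells with a height arc.
; Combat briefly shows a roll-results widget for attackers facing enemies, and the attacker ends the animation after a delay.
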(event `self.ReceiveBeginPlay`
  (`|ExecutionSequence`
    (:`then_0`
      (bind _returnvalue (`GameplayStatics.GetActorOfClass` "/Game/Board/BP_ChessBoard.BP_ChessBoard_C"))
      (set `self.Board` _returnvalue))
    (:`then_1`
      (message `/Game/UI/UI_ActorBoundWidget.SetBoundActor` (`WidgetComponent.GetWidget` (`self.Widget`)) self))))

(event `self.OnTypeChanged`
  (params (NewType :type "EFigureType Enum" :default "EFT_Pawn"))
  (`self.UpdateVisuals`))

(event `self.OnColorChanged`
  (params (NewColor :type "EChessColor Enum" :default "ECC_White"))
  (`self.UpdateVisuals`))

(event `UpdateFigureMesh`
  (bind (_value _returnvalue) (`BlueprintMapLibrary.Map_Find` (`self.FigureMeshByType`) (`self.FigureType`)))
  (if _returnvalue
    (`StaticMeshComponent.SetStaticMesh` (`self.FigureMesh`) _value)))

(event `UpdateDiceMesh`
  (bind (_value _returnvalue) (`BlueprintMapLibrary.Map_Find` (`self.DiceMeshByType`) (`self.FigureType`)))
  (if _returnvalue
    (`StaticMeshComponent.SetStaticMesh` (`self.DiceMesh`) _value)))

(event `UpdateVisuals`
  (`|ExecutionSequence`
    (:`then_1`
      (`self.UpdateDiceMesh`))
    (:`then_2`
      (`self.UpdateMaterials`))))

(event `UpdateMaterials`
  (bind _figurecolor (`self.FigureColor`))
  (`PrimitiveComponent.SetMaterial` (`self.FigureMesh`) 0 (select `EChessColor` _figurecolor :`ECC_White` (`self.WhiteMaterial`) :`ECC_Black` (`self.BlackMaterial`)))
  (`PrimitiveComponent.SetMaterial` (`self.DiceMesh`) 0 (select `EChessColor` _figurecolor :`ECC_White` (`self.BlackMaterial`) :`ECC_Black` (`self.WhiteMaterial`))))

(event `self.ReceiveActorOnClicked`
  (params (ButtonPressed :type "Key Structure"))
  (bind _asbp_player_controller (cast `/Game/Input/BP_PlayerController` (`GameplayStatics.GetPlayerController` 0)))
  (`/Game/Input/BP_PlayerController.HandleFigureClicked` _asbp_player_controller self))

(event `self.StartMovementAnimation`
  (params (Cell :type "GridCoords Structure (by ref)"))
  (bind _board (`self.Board`)
    (:`then`
      (`|ExecutionSequence`
        (:`then_0`
          (set `self.MoveStartTarget` (`self.K2_GetActorLocation`)))
        (:`then_1`
          (bind _result (`/Game/Board/BP_ChessBoard.GetPositionForCell` _board Cell))
          (set `self.MoveEndTarget` (+ _result (`self.K2_GetActorLocation` _board))))
        (:`then_2`
          (`TimelineComponent.SetPlayRate` (`self.Move`) (/ 2.0 (`self.MoveDuration`)))
          (bind (_direction _linearalpha _heightalpha) (`Timeline|Move` :!via `PlayFromStart`)
            (:`Update`
              (`self.K2_SetActorLocation` (+ (`|EaseFunction` "Linear" _linearalpha (`self.MoveStartTarget`) (`self.MoveEndTarget`)) (* (`self.MoveAnimHeight`) _heightalpha))))
            (:`Finished`
              (`self.EndMovementAnimation`))))))
    (:`else`
      (`KismetSystemLibrary.PrintString` "No board" true true (struct :`R` 1.0 :`G` 0.5 :`A` 1.0))
      (`KismetSystemLibrary.Delay` 1.0)
      (`self.EndMovementAnimation`))))

(event `ShowRollResults`
  (params (Duration :type "Float (double-precision)" :default 2.0))
  (`|ExecutionSequence`
    (:`then_0`
      (`SceneComponent.SetHiddenInGame` (`self.Widget`) false false))
    (:`then_1`
      (`KismetSystemLibrary.RetriggerableDelay` Duration)
      (`SceneComponent.SetHiddenInGame` (`self.Widget`) true false))))

(event `self.StartCombatAnimation`
  (params (Target :type "BaseChessFigure Object Reference") (bIsAttacker :type Boolean))
  (`|ExecutionSequence`
    (:`then_0`
      (if (and (`self.IsEnemy` Target) bIsAttacker)
        (`self.ShowRollResults` 2.0)))
    (:`then_1`
      (`KismetSystemLibrary.Delay` 2.0)
      (if bIsAttacker
        (`self.EndCombatAnimation`)))))

(event `self.OnMoveEnded`
  (bind _board (`self.Board`)
    (:`then`
      (bind _result (`/Game/Board/BP_ChessBoard.GetPositionForCell` _board (`self.CurrentPosition`)))
      (`self.K2_SetActorLocation` _result))
    (:`else`)))

(fn `DebugRollResults`
  (`KismetSystemLibrary.PrintString` (`KismetStringLibrary.Concat_StrStr` "Roll results are " (`KismetStringLibrary.Conv_IntToString` (`self.OurSavedRoll`)) " " (`KismetStringLibrary.Conv_IntToString` (`self.EnemySavedRoll`))) true true (struct :`R` 1.0 :`G` 0.5 :`A` 1.0)))

(fn `UserConstructionScript`)