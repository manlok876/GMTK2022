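; Chess game mode that populates the board with pieces from a board setup when play begins.
; It finds the BP_ChessBoard actor, then spawns each figure using a type-to-class map and its color.
; The board supplies cell positions, and black pieces are rotated 180 degrees.
; Each piece registers its starting cell, with on-screen errors for cell conflicts or missing classes.
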(event `self.ReceiveBeginPlay`
  (`|ExecutionSequence`
    (:`then_0`
      (bind _returnvalue (`GameplayStatics.GetActorOfClass` "/Game/Board/BP_ChessBoard.BP_ChessBoard_C"))
      (bind _output_get (set `self.Board` _returnvalue))
      (`/Engine/EditorBlueprintResources/StandardMacros.IsValid` _output_get
        (:`Is Not Valid`
          (`KismetSystemLibrary.PrintString` "No valid board" true true (struct :`R` 1.0 :`A` 1.0)))))
    (:`then_1`
      (`self.SpawnFiguresFromSetup` (`self.BoardSetup`)))))

(event `SpawnFiguresFromSetup`
  (params (BoardSetup :type "BoardSetup Object Reference"))
  (for _array_element (`BoardSetup.Figures` BoardSetup)
    (bind (_figure _position) (break `FigureSetupData` _array_element))
    (bind (_type _color) (break `FigureInfo` _figure))
    (bind (_value _returnvalue) (`BlueprintMapLibrary.Map_Find` (`self.FigureClassByType`) _type))
    (if _returnvalue
      (bind _returnvalue_2 (`self.GetTransformForFigureSetup` _array_element))
      (bind _returnvalue_3 (`|SpawnActorFromClass` _value _returnvalue_2 "AlwaysSpawn" "OverrideRootScale" null _color null))
      (`/Engine/EditorBlueprintResources/StandardMacros.IsValid` _returnvalue_3
        (:`Is Valid`
          (bind _returnvalue_4 (`BaseChessFigure.InitialPositionSet` _returnvalue_3 _position))
          (if (not _returnvalue_4)
            (bind (_row _column) (break `GridCoords` _position))
            (bind (_type_2 _color_2) (break `FigureInfo` _figure))
            (`KismetSystemLibrary.PrintString` (`KismetStringLibrary.Concat_StrStr` "Conflict at " (`KismetStringLibrary.Concat_StrStr` (`KismetStringLibrary.Conv_IntToString` _row) ", " (`KismetStringLibrary.Conv_IntToString` _column)) ", can't spawn " (`|GetEnumeratorNameAsString` _color_2) " " (`|GetEnumeratorNameAsString` _type_2)) true true (struct :`R` 1.0 :`A` 1.0)))))
      (else
        (`KismetSystemLibrary.PrintString` (`KismetStringLibrary.Concat_StrStr` "Class for type " (`|GetEnumeratorNameAsString` _type) " not found") true true (struct :`R` 1.0 :`A` 1.0))))))

(fn `GetTransformForFigureSetup`
  (params (Data :type "FigureSetupData Structure"))
  (returns (ReturnValue :type "Transform Structure"))
  (bind (_figure _position) (break `FigureSetupData` Data))
  (bind _board (`self.Board`)
    (:`then`
      (bind _result (`/Game/Board/BP_ChessBoard.GetPositionForCell` _board _position))
      (return (`KismetMathLibrary.MakeTransform` (+ _result (`self.K2_GetActorLocation` _board)) (`KismetMathLibrary.MakeRotator` 0.0 0.0 (select `EChessColor` (`.Color` (break `FigureInfo` _figure)) :`ECC_Black` 180.0 :!type "Float (single-precision)")))))
    (:`else`
      (return))))

(fn `UserConstructionScript`)